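; SideviewPlayer follows the FirstPersonPlayer as a side-view stand-in, and left-clicking shows the mouse cursor.
; Every Tick it finds all FirstPersonPlayer actors and moves itself to each one's Y and Z, raised by a fixed offset, with X locked at zero.
; A Launch event inverts the loop actor's gravity and turns it around, but its only call here is unreachable, as is a leftover LaunchCharacter branch.
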(event `Key|LeftMouseButton`
  (params (Key :type "Key Structure" :default "AnyKey"))
  (:`Pressed`
    (set `PlayerController.bShowMouseCursor` true (`GameplayStatics.GetPlayerController` 0))))

(event `self.ReceiveBeginPlay`)

(event `self.ReceiveActorBeginOverlap`
  (params (OtherActor :type "Actor Object Reference")))

(event `self.ReceiveTick`
  (params (DeltaSeconds :type "Float (single-precision)"))
  (bind _outactors (`GameplayStatics.GetAllActorsOfClass` "/Game/Blueprints/Player/FirstPersonPlayer.FirstPersonPlayer_C"))
  (for _array_element _outactors
    (`self.K2_SetActorLocation` (`KismetMathLibrary.MakeVector` 0.0 (.y (`self.K2_GetActorLocation` _array_element)) (+ (.z (`self.K2_GetActorLocation` _array_element)) 200.0)))))

(event `InputAction|Test`
  (params (Key :type "Key Structure" :default "AnyKey")))

(event `Launch`
  (set `CharacterMovementComponent.GravityScale` -0.2 (`Character.CharacterMovement` (stale `self.ReceiveTick` _array_element)))
  (`self.K2_AddActorWorldRotation` (stale `self.ReceiveTick` _array_element) (struct :`Pitch` 180.0) false false))

(fn `UserConstructionScript`)